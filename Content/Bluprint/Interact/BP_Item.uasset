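; BP_Item is an interactable world pickup that adds an item to the interacting actor's inventory.
; On interact, it passes its InventoryItemClass to AddItem on the Interactor's BPCInventory component, then destroys itself.
; It supplies "Collect Item" as its interaction prompt text, and its BeginPlay, overlap and Tick events are unused.
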(event `/Game/Bluprint/Interface/BPI_Interactable.Oninteract`
  (params (Interactor :type "/Game/Bluprint/ThirdPerson/Blueprints/BP_Player_Character Object Reference"))
  (`/Game/Bluprint/Inventory/BPC_Inventory.AddItem` (`/Game/Bluprint/ThirdPerson/Blueprints/BP_Player_Character.BPC_Inventory` Interactor) (`self.InventoryItemClass`))
  (`self.K2_DestroyActor`))

(fn `GetInteractText`
  (returns (ReturnText :type Text))
  (return "Collect Item"))

(fn `UserConstructionScript`
  (`parent.UserConstructionScript`))