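; Trigger zone actor that switches the player between a fixed camera and the third-person camera.
; When BP_Player_Character enters, it activates the Gameplay Camera rig on the referenced fixed camera actor and sets CameraStyle to Fixed.
; On exit, it activates the character's own GameplayCamera and restores the TPS style.
; Both switches use Push activation on player controller 0 and set the view target.
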(event `self.ReceiveActorBeginOverlap`
  (params (OtherActor :type "Actor Object Reference"))
  (bind _asbp_player_character (cast `/Game/Bluprint/ThirdPerson/Blueprints/BP_Player_Character` OtherActor))
  (`GameplayCameraComponentBase.ActivateCameraForPlayerController` (`/Game/Bluprint/Camera/BP_FixedCameraActor.GameplayCameraRig` (`self.FixeedCameraActor`)) (`GameplayStatics.GetPlayerController` 0) true "Push")
  (set `/Game/Bluprint/ThirdPerson/Blueprints/BP_Player_Character.CameraStyle` (struct :`TagName` "Camera.Style.Fixed") _asbp_player_character))

(event `self.ReceiveActorEndOverlap`
  (params (OtherActor :type "Actor Object Reference"))
  (bind _asbp_player_character (cast `/Game/Bluprint/ThirdPerson/Blueprints/BP_Player_Character` OtherActor))
  (`GameplayCameraComponentBase.ActivateCameraForPlayerController` (`/Game/Bluprint/ThirdPerson/Blueprints/BP_Player_Character.GameplayCamera` _asbp_player_character) (`GameplayStatics.GetPlayerController` 0) true "Push")
  (set `/Game/Bluprint/ThirdPerson/Blueprints/BP_Player_Character.CameraStyle` (struct :`TagName` "Camera.Style.TPS") _asbp_player_character))

(fn `UserConstructionScript`)